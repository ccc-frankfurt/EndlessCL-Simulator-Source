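; Sky handler Blueprint exposing events that control clouds, sun, skylight and time of day.
; LoadSkySphere caches the first BP_Sky_Sphere and BP_SunPosition; setters drive sky material parameters, SunLight and SkyLight intensity, and skylight recapture.
; SetTimeOfDay writes the time to BP_SunPosition and calls its UpdateSun.
; The handler's UpdateSun sets light temperature from a sun-height curve, but calls UpdateSunDirection only on the failed-cast branch.
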(event EventSetSunIntensity
  (params (Intesity :type Float%20%28single-precision%29))
  (Development|PrintString "Set Sun Intensity")
  (Rendering|Components|Light|SetIntensity (Variables|/Script/Engine.Light|GetLightComponent (Variables|Default|GetSunLight)) Intesity))

(event EventSetTimeOfDay
  (params (Houre :type Integer) (Minute :type Integer) (Seconds :type Integer))
  (bind _asbp_sun_position (Utilities|Casting|CastToBP_SunPosition (Variables|Default|GetSunPosition))
    (:then
      (Variables|/SunPosition/BP_SunPosition.BP_SunPosition_C|SetHours _asbp_sun_position Houre)
      (Variables|/SunPosition/BP_SunPosition.BP_SunPosition_C|SetMinutes _asbp_sun_position Minute)
      (Variables|/SunPosition/BP_SunPosition.BP_SunPosition_C|SetSeconds _asbp_sun_position Seconds)
      (Default|UpdateSun _asbp_sun_position))
    (:CastFailed
      (Development|PrintString "Cast Failed.."))))

(event EventSetSunBrightness
  (params (Brightness :type Float%20%28single-precision%29))
  (bind _asbp_sky_sphere (Utilities|Casting|CastToBP_Sky_Sphere (Variables|Default|GetSkySphere)))
  (Rendering|Material|SetScalarParameterValue (Variables|/Engine/EngineSky/BP_Sky_Sphere.BP_Sky_Sphere_C|GetSky%20material _asbp_sky_sphere) "Sun brightness" Brightness :!class /Script/Engine.MaterialInstanceDynamic))

(event EventSetCloudSpeed
  (params (CloudSpeed :type Float%20%28single-precision%29))
  (bind _asbp_sky_sphere (Utilities|Casting|CastToBP_Sky_Sphere (Variables|Default|GetSkySphere)))
  (Rendering|Material|SetScalarParameterValue (Variables|/Engine/EngineSky/BP_Sky_Sphere.BP_Sky_Sphere_C|GetSky%20material _asbp_sky_sphere) "Cloud Speed" CloudSpeed :!class /Script/Engine.MaterialInstanceDynamic))

(event EventReCaputreSkyLight
  (Class|SkyLightComponent|RecaptureSky (Variables|/Script/Engine.SkyLight|GetLightComponent (Variables|Default|GetSkyLight))))

(event EventSetCloudOpacity
  (params (CloudOpacity :type Float%20%28single-precision%29))
  (bind _asbp_sky_sphere (Utilities|Casting|CastToBP_Sky_Sphere (Variables|Default|GetSkySphere))
    (:then
      (Rendering|Material|SetScalarParameterValue (Variables|/Engine/EngineSky/BP_Sky_Sphere.BP_Sky_Sphere_C|GetSky%20material _asbp_sky_sphere) "Cloud opacity" CloudOpacity :!class /Script/Engine.MaterialInstanceDynamic))
    (:CastFailed
      (Development|PrintString "Cast Failed"))))

(event EventSetSkylightIntensity
  (params (Intensity :type Float%20%28single-precision%29))
  (Rendering|Components|Light|SetIntensity (Variables|/Script/Engine.SkyLight|GetLightComponent (Variables|Default|GetSkyLight)) Intensity))

(event EventUpdateSun
  (bind _asbp_sky_sphere (Utilities|Casting|CastToBP_Sky_Sphere (Variables|Default|GetSkySphere))
    (:then
      _)
    (:CastFailed
      (Default|UpdateSunDirection _asbp_sky_sphere)))
  (Class|LightComponent|SetTemperature (Variables|/Script/Engine.Light|GetLightComponent (Variables|/Engine/EngineSky/BP_Sky_Sphere.BP_Sky_Sphere_C|GetDirectional%20light%20actor _asbp_sky_sphere)) (Math|Curves|GetFloatValue (Variables|Default|GetTemparatureCurve) (Variables|/Engine/EngineSky/BP_Sky_Sphere.BP_Sky_Sphere_C|GetSun%20height _asbp_sky_sphere))))

(event EventLoadSkySphere
  ;[1 1 1] Get SkySphere
  (bind _outactors (Actor|GetAllActorsOfClass "/Engine/EngineSky/BP_Sky_Sphere.BP_Sky_Sphere_C"))
  (Variables|Default|SetSkySphere (Utilities|Array|Get(acopy) _outactors))
  ;[1 1 1] Get SunPoistion
  (bind _outactors_2 (Actor|GetAllActorsOfClass "/SunPosition/BP_SunPosition.BP_SunPosition_C"))
  (Variables|Default|SetSunPosition (Utilities|Array|Get(acopy) _outactors_2)))

(fn ConstructionScript)