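; Weather handler actor that exposes events for controlling rain and snow through the level's BP_WeatherTool.
; LoadWeatherHandler caches the first BP_WeatherTool actor found; each setter casts that reference and writes directly to its variables.
; Setters cover rain and snow toggles, particle brightness, density, rain impacts and ground material strength.
; Density and material strength apply to both rain and snow, while brightness affects only rain.
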(event EventBeginPlay)

(event Collision|EventActorBeginOverlap
  (params (OtherActor :type Actor%20Object%20Reference)))

(event EventTick
  (params (DeltaSeconds :type Float%20%28single-precision%29)))

(event EventSetIsRaining
  (params (IsRaining :type Boolean))
  (bind _asbp_weather_tool (Utilities|Casting|CastToBP_WeatherTool (Variables|Default|GetWeatherHandler)))
  (Variables|/Game/StormPack/Blueprints/BP_WeatherTool.BP_WeatherTool_C|SetEnable%20Rain _asbp_weather_tool IsRaining))

(event EventSetIsSnowing
  (params (IsSnowing :type Boolean))
  (bind _asbp_weather_tool (Utilities|Casting|CastToBP_WeatherTool (Variables|Default|GetWeatherHandler)))
  (Variables|/Game/StormPack/Blueprints/BP_WeatherTool.BP_WeatherTool_C|SetEnable%20Snow _asbp_weather_tool IsSnowing))

(event EventSetParticleBrightness
  (params (ParticleBrightenss :type Float%20%28single-precision%29))
  (bind _asbp_weather_tool (Utilities|Casting|CastToBP_WeatherTool (Variables|Default|GetWeatherHandler)))
  (Variables|/Game/StormPack/Blueprints/BP_WeatherTool.BP_WeatherTool_C|SetRain%20Brightness _asbp_weather_tool ParticleBrightenss))

(event EventSetParticleDensity
  (params (ParticleDensity :type Float%20%28single-precision%29))
  (bind _asbp_weather_tool (Utilities|Casting|CastToBP_WeatherTool (Variables|Default|GetWeatherHandler)))
  (bind _output_get (Variables|/Game/StormPack/Blueprints/BP_WeatherTool.BP_WeatherTool_C|SetRain%20Density _asbp_weather_tool ParticleDensity))
  (Variables|/Game/StormPack/Blueprints/BP_WeatherTool.BP_WeatherTool_C|SetSnow%20Density _asbp_weather_tool _output_get))

(event EventSetRainImpactDensity
  (params (RainImpactDensity :type Float%20%28single-precision%29))
  (bind _asbp_weather_tool (Utilities|Casting|CastToBP_WeatherTool (Variables|Default|GetWeatherHandler)))
  (Variables|/Game/StormPack/Blueprints/BP_WeatherTool.BP_WeatherTool_C|SetRain%20Impact%20Density _asbp_weather_tool RainImpactDensity))

(event EventSetMaterialAdjustmentStrength
  (params (MaterialAdjustmentStrength :type Float%20%28single-precision%29))
  (bind _asbp_weather_tool (Utilities|Casting|CastToBP_WeatherTool (Variables|Default|GetWeatherHandler)))
  (bind _output_get (Variables|/Game/StormPack/Blueprints/BP_WeatherTool.BP_WeatherTool_C|SetRain%20Ground%20Intensity _asbp_weather_tool MaterialAdjustmentStrength))
  (Variables|/Game/StormPack/Blueprints/BP_WeatherTool.BP_WeatherTool_C|SetSnow%20Ground%20Intensity _asbp_weather_tool _output_get))

(event EventLoadWeatherHandler
  ;[1 1 1] Get Access to WeatherHandler
  (bind _outactors (Actor|GetAllActorsOfClass "/Game/StormPack/Blueprints/BP_WeatherTool.BP_WeatherTool_C"))
  (Variables|Default|SetWeatherHandler (Utilities|Array|Get(acopy) _outactors)))

(fn ConstructionScript)