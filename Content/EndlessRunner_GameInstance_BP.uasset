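; Game Instance for the endless runner that relays level loading and simulation control events.
; Its events broadcast smooth level load (with level name and active widget), run simulation, end simulation and main menu load through matching Call dispatchers.
; Ending the simulation also prints a message and quits through the EXIT console command.
; An unconnected branch that would destroy all tiles through the game mode never runs.
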(event Custom|Event%20Smooth%20Load%20Level
  (params (LevelName :type String) (ActiveWidget :type User%20Widget%20Object%20Reference))
  (Default|CallSmoothLoadLevel LevelName ActiveWidget))

(event Custom|EndSimulation_Event
  (Default|CallEndSimulation)
  (Development|PrintString "GameInstance: EndSimulation Called")
  (Development|ExecuteConsoleCommand "EXIT" 0))

(event Custom|RunSimulation_Event
  (Default|CallRunSimulation))

(event Custom|LoadMainMenu_Event
  (Default|CallLoadMainMenu))